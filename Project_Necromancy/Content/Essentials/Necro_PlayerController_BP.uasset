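; Player controller that relays player input to the Necro_CamController pawn it controls, driving camera zoom, orbit and movement.
; Zoom in and out actions send a signed step to CameraZoom, while axis inputs pass their values to CameraOrbit, MoveForward and LeftRight.
; Each event casts the controlled pawn on every call and does nothing if it is another class, so the controller holds no movement or camera logic itself.
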(event Input|ActionEvents|InputActionCamZoomIn
  (params (Key :type Key%20Structure :default "None"))
  (:Pressed
    (bind _asnecro_cam_controller (Utilities|Casting|CastToNecro_CamController (Pawn|GetControlledPawn)))
    (Default|CameraZoom _asnecro_cam_controller -1.0)))

(event Input|ActionEvents|InputActionCamZoomOut
  (params (Key :type Key%20Structure :default "None"))
  (:Pressed
    (bind _asnecro_cam_controller (Utilities|Casting|CastToNecro_CamController (Pawn|GetControlledPawn)))
    (Default|CameraZoom _asnecro_cam_controller 1.0)))

(event Input|AxisEvents|InputAxisCameraOrbit
  (params (AxisValue :type Float%20%28single-precision%29))
  (bind _asnecro_cam_controller (Utilities|Casting|CastToNecro_CamController (Pawn|GetControlledPawn)))
  (Default|CameraOrbit _asnecro_cam_controller AxisValue))

(event Input|AxisEvents|InputAxisWalkforwards/Backwards
  (params (AxisValue :type Float%20%28single-precision%29))
  (bind _asnecro_cam_controller (Utilities|Casting|CastToNecro_CamController (Pawn|GetControlledPawn)))
  (Default|MoveForward _asnecro_cam_controller AxisValue))

(event Input|AxisEvents|InputAxisStrafeLeft/Right
  (params (AxisValue :type Float%20%28single-precision%29))
  (bind _asnecro_cam_controller (Utilities|Casting|CastToNecro_CamController (Pawn|GetControlledPawn)))
  (Default|Left/Right _asnecro_cam_controller AxisValue))

(fn ConstructionScript)